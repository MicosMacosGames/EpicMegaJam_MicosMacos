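; Player character that handles movement, pausing, interaction, death respawn and time travel between present and another era.
; Holding teleport ramps blur, camera shake and Wwise audio; releasing adds or subtracts the XY position of a "Teleporter"-tagged actor, with a cooldown.
; A per-tick camera trace finds InteractSphere components for the interaction HUD and input.
; BeginPlay creates HUDs and saves the current level; some abilities are level-gated, and F6 toggles non-shipping fly/no-collision mode.
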(event Custom|TogglePlayerMovements
  (params (CanMove :type Boolean) (CanRotate :type Boolean))
  ;[1 1 1] Enable/Disable Player Movements
  (Variables|Default|SetCanMove CanMove)
  (Variables|Default|SetCanRotate CanRotate))

(event Custom|QuitPauseEvent
  (bind _returnvalue (Game|GetPlayerController 0))
  ;[1 0.4583 0.4583] Pause Event & Pause Menu Navigation
  (Game|SetGamePaused false)
  (Input|SetInputModeGameOnly _returnvalue)
  (Variables|/Script/Engine.PlayerController|SetbShowMouseCursor _returnvalue false)
  (Widget|RemovefromParent (Variables|Default|GetPlayerPauseHUD)))

(event Custom|ChargeTimeTravel
  (params (StopCharge :type Boolean))
  (bind _returnvalue (Game|GetPlayerController 0))
  ;[0.3848 1 0.7098] The same Teleport put keeping pressed (2 events now!)
  (Class|AkGameplayStatics|PostEvent "/Game/WwiseAudio/Events/Default_Work_Unit/Gameplay/tp_start.tp_start" self)
  (bind _returnvalue_2 (Rendering|Material|GetScalarParameterValue "/Game/Assets/Materials/RadialBlurMaterial/BlurMatParameters.BlurMatParameters" "BlurRadius" :!class /Script/Engine.KismetMaterialLibrary))
  (bind _returnvalue_3 (Rendering|Material|GetScalarParameterValue "/Game/Assets/Materials/RadialBlurMaterial/BlurMatParameters.BlurMatParameters" "BlurDensity" :!class /Script/Engine.KismetMaterialLibrary))
  (bind _returnvalue_4 (Rendering|Material|GetScalarParameterValue "/Game/Assets/Materials/RadialBlurMaterial/BlurMatParameters.BlurMatParameters" "BlurAmount" :!class /Script/Engine.KismetMaterialLibrary))
  (bind (_direction _newtrack_0) (Timeline|Timeline_1 PlayFromStart)
    (:Update
      (Rendering|Material|SetScalarParameterValue "/Game/Assets/Materials/RadialBlurMaterial/BlurMatParameters.BlurMatParameters" "BlurRadius" (Math|Float|Lerp _returnvalue_2 1.0 _newtrack_0) :!class /Script/Engine.KismetMaterialLibrary)
      (Rendering|Material|SetScalarParameterValue "/Game/Assets/Materials/RadialBlurMaterial/BlurMatParameters.BlurMatParameters" "BlurDensity" (Math|Float|Lerp _returnvalue_3 0.0 _newtrack_0) :!class /Script/Engine.KismetMaterialLibrary)
      (Rendering|Material|SetScalarParameterValue "/Game/Assets/Materials/RadialBlurMaterial/BlurMatParameters.BlurMatParameters" "BlurAmount" (Math|Float|Lerp _returnvalue_4 2.0 _newtrack_0) :!class /Script/Engine.KismetMaterialLibrary)
      (Class|PlayerController|ClientPlayCameraShake _returnvalue "/Game/Blueprints/Effects_BPs/CameraShake_BP.CameraShake_BP_C" 0.05 "CameraLocal" "0, 0, 0")
      (Class|AkGameplayStatics|SetRTPCValue "/Game/WwiseAudio/Game_Parameters/Default_Work_Unit/tp_cast_volume.tp_cast_volume" _newtrack_0 0 self))
    (:Finished
      (switch Utilities|FlowControl|Switch|SwitchonETimelineDirection _direction
        (:Forward
          (Class|PlayerController|ClientPlayCameraShake _returnvalue "/Game/Blueprints/Effects_BPs/CameraShake_BP.CameraShake_BP_C" 0.1 "CameraLocal" "0, 0, 0" :!label _label)
          (Utilities|FlowControl|Delay 0.1)
          (if (Variables|Default|GetKeepShaking)
            (goto _label)
            (else
              (Variables|Default|SetKeepShaking true))))))))

(event Custom|DeathEvent
  ;[0.8625 0.5649 1] Death Event
  (Class|AkGameplayStatics|PostEvent "/Game/WwiseAudio/Events/Default_Work_Unit/Music/play_death_music.play_death_music" self)
  (Widget|SetVisibility (Variables|Default|GetPlayerGameplayHUD) "Hidden")
  (bind _returnvalue (Game|GetCurrentLevelName true))
  (Variables|/Game/Blueprints/GameInstance.GameInstance_C|SetCurrentLevel (.AsGame%20Instance (Utilities|Casting|CastToGameInstance (Game|GetGameInstance))) (Utilities|String|StringToName _returnvalue))
  (CallFunction|TogglePlayerMovements false false)
  (bind _returnvalue_2 (UserInterface|CreateWidget "/Game/Blueprints/HUD_BPs/Fades/BlackFadeOut.BlackFadeOut_C"))
  (UserInterface|Viewport|AddtoViewport _returnvalue_2 5)
  (Utilities|FlowControl|Delay 2.0)
  (bind _returnvalue_3 (Game|GetCurrentLevelName true))
  (if (and (Utilities|Enum|Equal(Enum) _returnvalue_3 "Level4Map_2") (Variables|Default|GetReachedCheckpointLevel4))
    (Transformation|SetActorLocation (Variables|Default|GetCheckpointLevel4Location) false true)
    (else
      (bind _outactors (Actor|GetAllActorsOfClass "/Script/Engine.PlayerStart"))
      (Transformation|SetActorLocation (Transformation|GetActorLocation (Utilities|Array|Get(acopy) _outactors)) false true)))
  (bind _returnvalue_4 (UserInterface|CreateWidget "/Game/Blueprints/HUD_BPs/Fades/BlackFadeIn.BlackFadeIn_C"))
  (UserInterface|Viewport|AddtoViewport _returnvalue_4 5)
  (Utilities|FlowControl|Delay 2.0)
  (CallFunction|TogglePlayerMovements true true)
  (Variables|Default|SetIsInPresent true))

(event Custom|TimeTravelEvent
  (bind _returnvalue (Transformation|GetActorLocation))
  ;[0.3848 1 0.7098] Teleport Event - It gets the first object with tag "Teleporter". Then it teleports the player to Teleporter pos. + (or -) player pos.
  (bind _outactors (Actor|GetAllActorswithTag "Teleporter"))
  (if (> (Utilities|Array|Length _outactors) 0)
    (bind (_direction _newtrack_0) (Timeline|Timeline_0 PlayFromStart)
      (:Update
        (Rendering|Material|SetScalarParameterValue "/Game/Assets/Materials/RadialBlurMaterial/BlurMatParameters.BlurMatParameters" "BlurRadius" (Math|Float|Lerp 0.0 1.0 _newtrack_0) :!class /Script/Engine.KismetMaterialLibrary)
        (Rendering|Material|SetScalarParameterValue "/Game/Assets/Materials/RadialBlurMaterial/BlurMatParameters.BlurMatParameters" "BlurDensity" (Math|Float|Lerp 4.0 0.0 _newtrack_0) :!class /Script/Engine.KismetMaterialLibrary)
        (Rendering|Material|SetScalarParameterValue "/Game/Assets/Materials/RadialBlurMaterial/BlurMatParameters.BlurMatParameters" "BlurAmount" (Math|Float|Lerp 0.0 2.0 _newtrack_0) :!class /Script/Engine.KismetMaterialLibrary))
      (:Finished
        (switch Utilities|FlowControl|Switch|SwitchonETimelineDirection _direction
          (:Forward
            (bind _returnvalue_2 (UserInterface|CreateWidget "/Game/Blueprints/HUD_BPs/Fades/FastWhiteFadeIn.FastWhiteFadeIn_C"))
            (UserInterface|Viewport|AddtoViewport _returnvalue_2 0)
            (Utilities|FlowControl|Delay 0.1)
            (if (Variables|Default|GetIsInPresent)
              (bind _returnvalue_3 (Transformation|Teleport (+ _returnvalue (Math|Vector|MakeVector (.X (Math|Vector|BreakVector (Transformation|GetActorLocation (Utilities|Array|Get(acopy) _outactors)))) (.Y (Math|Vector|BreakVector (Transformation|GetActorLocation (Utilities|Array|Get(acopy) _outactors)))) 0.0)) "0, 0, 0"))
              (if _returnvalue_3
                (Variables|Default|SetIsInPresent (not (Variables|Default|GetIsInPresent)) :!label _label)
                (Utilities|FlowControl|DoOnce false :!label _label_2
                  (:Completed
                    (Components|Timeline|ReversefromEnd (Variables|Default|GetTimeline_0))
                    (goto _label_2 Reset))))
              (else
                (bind _returnvalue_4 (Transformation|Teleport (- _returnvalue (Math|Vector|MakeVector (.X (Math|Vector|BreakVector (Transformation|GetActorLocation (Utilities|Array|Get(acopy) _outactors)))) (.Y (Math|Vector|BreakVector (Transformation|GetActorLocation (Utilities|Array|Get(acopy) _outactors)))) 0.0)) "0, 0, 0"))
                (if _returnvalue_4
                  (goto _label))))))))))

(event Custom|PressedTimeTravel
  (bind _returnvalue (Transformation|GetActorLocation))
  ;[0.3848 1 0.7098] The same Teleport put keeping pressed (2 events now!)
  (Variables|Default|SetPlayerRotationBeforeTeleport (Transformation|GetActorRotation))
  (Class|AkGameplayStatics|PostEvent "/Game/WwiseAudio/Events/Default_Work_Unit/Gameplay/tp_end.tp_end" self)
  (Variables|Default|SetKeepShaking false)
  (bind _outactors (Actor|GetAllActorswithTag "Teleporter"))
  (if (> (Utilities|Array|Length _outactors) 0)
    (bind _returnvalue_2 (UserInterface|CreateWidget "/Game/Blueprints/HUD_BPs/Fades/FastWhiteFadeIn.FastWhiteFadeIn_C"))
    (UserInterface|Viewport|AddtoViewport _returnvalue_2 0)
    (Utilities|FlowControl|Delay 0.1)
    (if (Variables|Default|GetIsInPresent)
      (bind _returnvalue_3 (Transformation|Teleport (+ _returnvalue (Math|Vector|MakeVector (.X (Math|Vector|BreakVector (Transformation|GetActorLocation (Utilities|Array|Get(acopy) _outactors)))) (.Y (Math|Vector|BreakVector (Transformation|GetActorLocation (Utilities|Array|Get(acopy) _outactors)))) 0.0)) "0, 0, 0"))
      (if _returnvalue_3
        (Variables|Default|SetIsInPresent (not (Variables|Default|GetIsInPresent)) :!label _label)
        (Transformation|SetActorRotation (Variables|Default|GetPlayerRotationBeforeTeleport))
        (bind _returnvalue_4 (Rendering|Material|GetScalarParameterValue "/Game/Assets/Materials/RadialBlurMaterial/BlurMatParameters.BlurMatParameters" "BlurRadius" :!class /Script/Engine.KismetMaterialLibrary))
        (bind _returnvalue_5 (Rendering|Material|GetScalarParameterValue "/Game/Assets/Materials/RadialBlurMaterial/BlurMatParameters.BlurMatParameters" "BlurDensity" :!class /Script/Engine.KismetMaterialLibrary))
        (bind _returnvalue_6 (Rendering|Material|GetScalarParameterValue "/Game/Assets/Materials/RadialBlurMaterial/BlurMatParameters.BlurMatParameters" "BlurAmount" :!class /Script/Engine.KismetMaterialLibrary))
        (bind _newtrack_0 (Timeline|Timeline_2 PlayFromStart)
          (:Update
            (Rendering|Material|SetScalarParameterValue "/Game/Assets/Materials/RadialBlurMaterial/BlurMatParameters.BlurMatParameters" "BlurRadius" (Math|Float|Lerp _returnvalue_4 0.0 _newtrack_0) :!class /Script/Engine.KismetMaterialLibrary)
            (Rendering|Material|SetScalarParameterValue "/Game/Assets/Materials/RadialBlurMaterial/BlurMatParameters.BlurMatParameters" "BlurDensity" (Math|Float|Lerp _returnvalue_5 4.0 _newtrack_0) :!class /Script/Engine.KismetMaterialLibrary)
            (Rendering|Material|SetScalarParameterValue "/Game/Assets/Materials/RadialBlurMaterial/BlurMatParameters.BlurMatParameters" "BlurAmount" (Math|Float|Lerp _returnvalue_6 0.0 _newtrack_0) :!class /Script/Engine.KismetMaterialLibrary)
            (Class|PlayerController|ClientPlayCameraShake (Game|GetPlayerController 0) "/Game/Blueprints/Effects_BPs/CameraShake_BP.CameraShake_BP_C" 0.05 "CameraLocal" "0, 0, 0"))
          (:Finished
            (Audio|Components|Audio|Stop (Variables|Default|GetTimeline_1)))))
      (else
        (bind _returnvalue_7 (Transformation|Teleport (- _returnvalue (Math|Vector|MakeVector (.X (Math|Vector|BreakVector (Transformation|GetActorLocation (Utilities|Array|Get(acopy) _outactors)))) (.Y (Math|Vector|BreakVector (Transformation|GetActorLocation (Utilities|Array|Get(acopy) _outactors)))) 0.0)) "0, 0, 0"))
        (if _returnvalue_7
          (goto _label))))))

(event EventBeginPlay
  (bind _returnvalue (Game|GetPlayerController 0))
  ;[1 1 1] BeginPlay Actions (Fade In, HUD Creation, ...)
  (Input|SetInputModeGameOnly _returnvalue)
  (Variables|/Script/Engine.PlayerController|SetbShowMouseCursor _returnvalue false)
  (bind _returnvalue_2 (UserInterface|CreateWidget "/Game/Blueprints/HUD_BPs/Fades/WhiteFadeIn.WhiteFadeIn_C"))
  (UserInterface|Viewport|AddtoViewport _returnvalue_2 3)
  (bind _returnvalue_3 (UserInterface|CreateWidget "/Game/Blueprints/HUD_BPs/GameHUD.GameHUD_C"))
  (bind _output_get (Variables|Default|SetPlayerGameplayHUD _returnvalue_3))
  (UserInterface|Viewport|AddtoViewport _output_get 2)
  (bind _returnvalue_4 (UserInterface|CreateWidget "/Game/Blueprints/HUD_BPs/InteractionHUD.InteractionHUD_C"))
  (bind _output_get_2 (Variables|Default|SetPlayerInteractionHUD _returnvalue_4))
  (UserInterface|Viewport|AddtoViewport _output_get_2 1)
  (Game|GetCurrentLevelName true)
  (Utilities|FlowControl|Delay 1.0)
  (bind _returnvalue_5 (SaveGame|DoesSaveGameExist "OwnSaveGame"))
  (if _returnvalue_5
    (bind _returnvalue_6 (SaveGame|LoadGamefromSlot "OwnSaveGame"))
    (Variables|Default|SetPlayerSaveGame _returnvalue_6)
    (else
      (bind _returnvalue_7 (SaveGame|CreateSaveGameObject "/Game/Blueprints/SaveGame_BP.SaveGame_BP_C"))
      (Variables|Default|SetPlayerSaveGame _returnvalue_7)))
  (bind _returnvalue_8 (Game|GetCurrentLevelName true))
  (Variables|/Game/Blueprints/SaveGame_BP.SaveGame_BP_C|SetLastPlayedLevel (.AsSave%20Game%20BP (Utilities|Casting|CastToSaveGame_BP (Variables|Default|GetPlayerSaveGame))) (Utilities|String|StringToName _returnvalue_8))
  (SaveGame|SaveGametoSlot (.AsSave%20Game%20BP (Utilities|Casting|CastToSaveGame_BP (Variables|Default|GetPlayerSaveGame))) "OwnSaveGame"))

(event EventTick
  (params (DeltaSeconds :type Float%20%28single-precision%29))
  ;[1 1 1] BeginPlay Actions (Fade In, HUD Creation, ...)
  (CallFunction|CheckLookatActor))

(event Input|ActionEvents|InputActionJump
  (params (Key :type Key%20Structure :default "None"))
  ;[0.6533 0.8108 1] Move & Jump
  (:Pressed
    (bind _returnvalue (Game|GetCurrentLevelName true))
    (if (not (Utilities|Enum|Equal(Enum) _returnvalue "Level6"))
      (Utilities|FlowControl|DoOnce false :!label _label
        (:Completed
          (if (Variables|Default|GetCanMove)
            (Character|Jump))))))
  (:Released
    (bind _returnvalue_2 (Game|GetCurrentLevelName true))
    (if (not (Utilities|Enum|Equal(Enum) _returnvalue_2 "Level6"))
      (Character|StopJumping)
      (Utilities|FlowControl|Delay 0.7)
      (goto _label Reset))))

(event Input|ActionEvents|InputActionE_Interact
  (params (Key :type Key%20Structure :default "None"))
  (bind _actorlookingat (Variables|Default|GetActorLookingAt))
  ;[1 1 1] Interaction Event
  (:Pressed
    (Utilities|IsValid _actorlookingat
      (:Is%20Valid
        (Class|InteractionInterfaceBP|InteractFunction(Message) _actorlookingat))))
  (:Released
    (Utilities|IsValid _actorlookingat
      (:Is%20Valid
        (Class|InteractionInterfaceBP|DeInteractFunction(Message) _actorlookingat)))))

(event Input|ActionEvents|InputActionPause
  (params (Key :type Key%20Structure :default "None"))
  (bind _returnvalue (Game|GetPlayerController 0))
  ;[1 0.4583 0.4583] Pause Event & Pause Menu Navigation
  (:Pressed
    (if (Game|IsGamePaused)
      (if (Variables|Default|GetFocusGameReturnButton)
        (Default|EventCustomClick (Variables|/Game/Blueprints/HUD_BPs/PauseHUD.PauseHUD_C|GetReturnToGameCustomButton (Variables|Default|GetPlayerPauseHUD)))
        (else
          (Default|EventCustomClick (Variables|/Game/Blueprints/HUD_BPs/PauseHUD.PauseHUD_C|GetExitToMenuCustomButton (Variables|Default|GetPlayerPauseHUD)))))
      (else
        (Game|SetGamePaused true)
        (bind _returnvalue_2 (UserInterface|CreateWidget "/Game/Blueprints/HUD_BPs/PauseHUD.PauseHUD_C"))
        (bind _output_get (Variables|Default|SetPlayerPauseHUD _returnvalue_2))
        (UserInterface|Viewport|AddtoViewport _output_get 0)
        (Input|SetInputModeGameandUI _returnvalue 0 "DoNotLock" true)
        (Variables|/Script/Engine.PlayerController|SetbShowMouseCursor _returnvalue true)
        (Default|EventCustomHover (Variables|/Game/Blueprints/HUD_BPs/PauseHUD.PauseHUD_C|GetReturnToGameCustomButton (Variables|Default|GetPlayerPauseHUD)) false)
        (Variables|Default|SetFocusGameReturnButton true)))))

(event Input|ActionEvents|InputActionMenuUp
  (params (Key :type Key%20Structure :default "None"))
  (bind _playerpausehud (Variables|Default|GetPlayerPauseHUD))
  ;[1 0.4583 0.4583] Pause Event & Pause Menu Navigation
  (:Pressed
    (if (Game|IsGamePaused)
      (if (Variables|Default|GetFocusGameReturnButton)
        (Default|EventCustomHover (Variables|/Game/Blueprints/HUD_BPs/PauseHUD.PauseHUD_C|GetExitToMenuCustomButton _playerpausehud) true)
        (Variables|Default|SetFocusGameReturnButton false)
        (else
          (Default|EventCustomHover (Variables|/Game/Blueprints/HUD_BPs/PauseHUD.PauseHUD_C|GetReturnToGameCustomButton _playerpausehud) true)
          (Variables|Default|SetFocusGameReturnButton true))))))

(event Input|ActionEvents|InputActionMenuDown
  (params (Key :type Key%20Structure :default "None"))
  (bind _playerpausehud (Variables|Default|GetPlayerPauseHUD))
  ;[1 0.4583 0.4583] Pause Event & Pause Menu Navigation
  (:Pressed
    (if (Game|IsGamePaused)
      (if (Variables|Default|GetFocusGameReturnButton)
        (Default|EventCustomHover (Variables|/Game/Blueprints/HUD_BPs/PauseHUD.PauseHUD_C|GetExitToMenuCustomButton _playerpausehud) true)
        (Variables|Default|SetFocusGameReturnButton false)
        (else
          (Default|EventCustomHover (Variables|/Game/Blueprints/HUD_BPs/PauseHUD.PauseHUD_C|GetReturnToGameCustomButton _playerpausehud) true)
          (Variables|Default|SetFocusGameReturnButton true))))))

(event Input|ActionEvents|InputActionPlayerTeleport
  (params (Key :type Key%20Structure :default "None"))
  (bind _returnvalue (Game|GetPlayerCharacter 0))
  (bind _asplayer_bp (Utilities|Casting|CastToPlayer_BP _returnvalue))
  ;[0.6533 0.8108 1] Move & Jump
  (:Pressed
    (bind _returnvalue_2 (Game|GetCurrentLevelName true))
    (if (not (Utilities|Enum|Equal(Enum) _returnvalue_2 "Lvl1"))
      (Utilities|FlowControl|DoOnce false :!label _label
        (:Completed
          (Variables|Default|SetTravelNow true)
          (CallFunction|ChargeTimeTravel _asplayer_bp false)))))
  (:Released
    (bind _returnvalue_3 (Game|GetCurrentLevelName true))
    (if (not (Utilities|Enum|Equal(Enum) _returnvalue_3 "Lvl1"))
      (if (Variables|Default|GetTravelNow)
        (CallFunction|PressedTimeTravel _asplayer_bp)
        (Variables|Default|SetTravelNow false)
        (Utilities|FlowControl|Delay (Variables|Default|GetTeleportCooldown))
        (goto _label Reset)))))

(event Input|ActionEvents|InputActionMenuBack
  (params (Key :type Key%20Structure :default "None"))
  (bind _returnvalue (Game|GetPlayerController 0))
  ;[1 0.4583 0.4583] Pause Event & Pause Menu Navigation
  (:Pressed
    (if (Game|IsGamePaused)
      (Game|SetGamePaused false)
      (Input|SetInputModeGameOnly _returnvalue)
      (Variables|/Script/Engine.PlayerController|SetbShowMouseCursor _returnvalue false)
      (Widget|RemovefromParent (Variables|Default|GetPlayerPauseHUD)))))

(event Input|ActionEvents|InputActionSprint
  (params (Key :type Key%20Structure :default "None"))
  ;[0.6533 0.8108 1] Move & Jump
  (:Pressed
    (bind _returnvalue (Game|GetCurrentLevelName true))
    (if (not (Utilities|Enum|Equal(Enum) _returnvalue "Level6"))
      (if (Variables|Default|GetMovingForward)
        (Variables|/Script/Engine.CharacterMovementComponent|SetMaxWalkSpeed (Variables|/Script/Engine.Character|GetCharacterMovement (Game|GetPlayerCharacter 0)) 6e+02))))
  (:Released
    (bind _returnvalue_2 (Game|GetCurrentLevelName true))
    (if (not (Utilities|Enum|Equal(Enum) _returnvalue_2 "Level6"))
      (Variables|/Script/Engine.CharacterMovementComponent|SetMaxWalkSpeed (Variables|/Script/Engine.Character|GetCharacterMovement (Game|GetPlayerCharacter 0)) 3e+02))))

(event Input|ActionEvents|InputActionMenuSelect
  (params (Key :type Key%20Structure :default "None"))
  (bind _playerpausehud (Variables|Default|GetPlayerPauseHUD))
  ;[1 0.4583 0.4583] Pause Event & Pause Menu Navigation
  (:Pressed
    (if (Game|IsGamePaused)
      (if (Variables|Default|GetFocusGameReturnButton)
        (Default|EventCustomClick (Variables|/Game/Blueprints/HUD_BPs/PauseHUD.PauseHUD_C|GetReturnToGameCustomButton _playerpausehud))
        (else
          (Default|EventCustomClick (Variables|/Game/Blueprints/HUD_BPs/PauseHUD.PauseHUD_C|GetExitToMenuCustomButton _playerpausehud)))))))

(event Input|AxisEvents|InputAxisMoveForward
  (params (AxisValue :type Float%20%28single-precision%29))
  (bind _returnvalue (> AxisValue 0.0))
  ;[0.6533 0.8108 1] Move & Jump
  (if (Variables|Default|GetCanMove)
    (bind _output_get (Variables|Default|SetMovingForward _returnvalue))
    (if _output_get
      _
      (else
        (Variables|/Script/Engine.CharacterMovementComponent|SetMaxWalkSpeed (Variables|/Script/Engine.Character|GetCharacterMovement (Game|GetPlayerCharacter 0)) 3e+02)))
    (Pawn|Input|AddMovementInput (Transformation|GetActorForwardVector) (Math|Float|SelectFloat AxisValue (* AxisValue 0.6) _returnvalue) false)
    (if (or (>= AxisValue 0.99) (<= AxisValue -0.99))
      (Transformation|SetActorRotation (Math|Interpolation|RInterpTo (Transformation|GetActorRotation) (Math|Rotator|MakeRotator 0.0 0.0 (.Yaw (Math|Rotator|BreakRotator (Pawn|GetControlRotation :!class /Script/Engine.Pawn)))) (Utilities|Time|GetWorldDeltaSeconds) 7.0)))))

(event Input|AxisEvents|InputAxisMoveRight
  (params (AxisValue :type Float%20%28single-precision%29))
  ;[0.6533 0.8108 1] Move & Jump
  (if (Variables|Default|GetCanMove)
    (Pawn|Input|AddMovementInput (Transformation|GetActorRightVector) AxisValue false)
    (if (or (>= AxisValue 0.9) (<= AxisValue -0.9))
      (Transformation|SetActorRotation (Math|Interpolation|RInterpTo (Transformation|GetActorRotation) (Math|Rotator|MakeRotator 0.0 0.0 (.Yaw (Math|Rotator|BreakRotator (Pawn|GetControlRotation :!class /Script/Engine.Pawn)))) (Utilities|Time|GetWorldDeltaSeconds) 7.0)))))

(event Input|AxisEvents|InputAxisGodFly
  (params (AxisValue :type Float%20%28single-precision%29))
  ;[0.5262 1 0.7367] GodMode
  (if (Variables|Default|GetGodMode)
    (Pawn|Input|AddMovementInput (Transformation|GetActorUpVector) AxisValue false)))

(event Input|AxisEvents|InputAxisMouseLookUp
  (params (AxisValue :type Float%20%28single-precision%29))
  ;[1 0.821 0.4532] Look Around
  (if (Variables|Default|GetCanRotate)
    (Pawn|Input|AddControllerPitchInput AxisValue)))

(event Input|AxisEvents|InputAxisGamepadLookUp
  (params (AxisValue :type Float%20%28single-precision%29))
  ;[1 0.821 0.4532] Look Around
  (if (Variables|Default|GetCanRotate)
    (Pawn|Input|AddControllerPitchInput (* AxisValue (Utilities|Time|GetWorldDeltaSeconds) (Variables|Default|GetLookAroundSpeed)))))

(event Input|AxisEvents|InputAxisGamepadTurnAround
  (params (AxisValue :type Float%20%28single-precision%29))
  ;[1 0.821 0.4532] Look Around
  (if (Variables|Default|GetCanRotate)
    (Pawn|Input|AddControllerYawInput (* AxisValue (Utilities|Time|GetWorldDeltaSeconds) (Variables|Default|GetLookAroundSpeed)))))

(event Input|AxisEvents|InputAxisMouseTurnAround
  (params (AxisValue :type Float%20%28single-precision%29))
  ;[1 0.821 0.4532] Look Around
  (if (Variables|Default|GetCanRotate)
    (Pawn|Input|AddControllerYawInput AxisValue)))

(event Input|KeyboardEvents|F6
  (params (Key :type Key%20Structure :default "None"))
  (bind _charactermovement (Variables|Character|GetCharacterMovement))
  (bind _capsulecomponent (Variables|Collision|GetCapsuleComponent))
  (bind _playergameplayhud (Variables|Default|GetPlayerGameplayHUD))
  (bind _asgame_hud (Utilities|Casting|CastToGameHUD _playergameplayhud))
  (bind _godmodetext (Variables|/Game/Blueprints/HUD_BPs/GameHUD.GameHUD_C|GetGodModeText _asgame_hud))
  ;[0.5262 1 0.7367] GodMode
  (:Pressed
    (if (not (Class|KismetSystemLibrary|IsPackagedforDistribution))
      (Development|ExecuteConsoleCommand "Stat UNIT" 0)
      (Development|ExecuteConsoleCommand "show Collision" 0)
      (if (Variables|Default|GetGodMode)
        (Pawn|Components|CharacterMovement|SetMovementMode _charactermovement "MOVE_Walking" 0)
        (Collision|SetCollisionEnabled _capsulecomponent "QueryAndPhysics")
        (Variables|Default|SetGodMode false)
        (Widget|SetVisibility _godmodetext "Hidden")
        (else
          (Pawn|Components|CharacterMovement|SetMovementMode _charactermovement "MOVE_Flying" 0)
          (Collision|SetCollisionEnabled _capsulecomponent "NoCollision")
          (Variables|Default|SetGodMode true)
          (Widget|SetVisibility _godmodetext "Visible"))))))

(fn ConstructionScript)

(fn CheckLookatActor
  (bind _returnvalue (Game|GetPlayerCameraManager 0))
  (bind _returnvalue_2 (Camera|GetCameraLocation _returnvalue))
  (bind (_outhit _returnvalue_3) (Collision|LineTraceByChannel _returnvalue_2 (+ _returnvalue_2 (* (Transformation|GetActorForwardVector _returnvalue) (Variables|Default|GetLookAtLength))) "TraceTypeQuery2" false 0 "None" true "(R=1.000000,G=0.000000,B=0.000000,A=1.000000)" "(R=0.000000,G=1.000000,B=0.000000,A=1.000000)" 2.0))
  (if _returnvalue_3
    (if (Components|ComponentHasTag (.HitComponent (Collision|BreakHitResult _outhit)) "InteractSphere")
      (if (== (Variables|Default|GetNewComponentLookingAt) (.HitComponent (Collision|BreakHitResult _outhit)))
        _
        (else
          (Utilities|IsValid (Variables|Default|GetNewComponentLookingAt)
            (:Is%20Valid
              (Default|ResetShowHUDDoOnce (.AsChild%20Interaction%20BP (Utilities|Casting|CastToChildInteractionBP (Components|GetOwner (Variables|Default|GetNewComponentLookingAt))))))
            (:Is%20Not%20Valid
              _))))
      (Variables|Default|SetNewComponentLookingAt (.HitComponent (Collision|BreakHitResult _outhit)))
      (Variables|Default|SetActorLookingAt (.HitActor (Collision|BreakHitResult _outhit)))
      (Default|ShowInteractionHUD (.AsChild%20Interaction%20BP (Utilities|Casting|CastToChildInteractionBP (Components|GetOwner (.HitComponent (Collision|BreakHitResult _outhit))))))
      (else
        (Utilities|IsValid (Variables|Default|GetActorLookingAt) :!label _label
          (:Is%20Valid
            (Default|ResetShowHUDDoOnce (.AsChild%20Interaction%20BP (Utilities|Casting|CastToChildInteractionBP (Components|GetOwner (Variables|Default|GetNewComponentLookingAt))))))
          (:Is%20Not%20Valid
            _))
        (Variables|Default|SetActorLookingAt 0)
        (Variables|Default|SetNewComponentLookingAt 0)
        (Default|HideHUD (Variables|Default|GetPlayerInteractionHUD))))
    (else
      (goto _label))))