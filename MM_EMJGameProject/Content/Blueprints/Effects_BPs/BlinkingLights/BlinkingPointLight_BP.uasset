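; BlinkingPointLight_BP makes a referenced light actor, LightToBlink, blink from BeginPlay in one of two modes.
; With CurveControlledBlink set, a timeline with its play rate derived from BlinkPeriod samples LightIntesityCurve to scale the light's initial intensity.
; Otherwise, an endless delay loop hides and shows the whole light actor, drawing random off and on durations from their respective ranges.
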(event EventBeginPlay
  (bind _lighttoblink (Variables|Default|GetLightToBlink))
  (bind _onrandomrange (Variables|Default|GetOnRandomRange))
  (bind _offrandomrange (Variables|Default|GetOffRandomRange))
  (bind (_x _y) (Math|Vector2D|BreakVector2D _onrandomrange))
  (bind (_x_2 _y_2) (Math|Vector2D|BreakVector2D _offrandomrange))
  (if (Variables|Default|GetCurveControlledBlink)
    (Variables|Default|SetInitialLightIntesity (Variables|/Script/Engine.LightComponentBase|GetIntensity (Variables|/Script/Engine.Light|GetLightComponent (Variables|Default|GetLightToBlink))))
    (Components|Timeline|SetPlayRate (Variables|Default|GetTimeline_0) (/ 1.0 (Variables|Default|GetBlinkPeriod)))
    (bind _newtrack_0 (Timeline|Timeline_0 PlayFromStart)
      (:Update
        (Rendering|Components|Light|SetIntensity (Variables|/Script/Engine.Light|GetLightComponent (Variables|Default|GetLightToBlink)) (* (Math|Curves|GetFloatValue (Variables|Default|GetLightIntesityCurve) _newtrack_0) (Variables|Default|GetInitialLightIntesity)))))
    (else
      (Rendering|SetActorHiddenInGame _lighttoblink true :!label _label)
      (Utilities|FlowControl|Delay (Math|Random|RandomFloatinRange _x_2 _y_2))
      (Rendering|SetActorHiddenInGame _lighttoblink false)
      (Utilities|FlowControl|Delay (Math|Random|RandomFloatinRange _x _y))
      (goto _label))))

(fn ConstructionScript)