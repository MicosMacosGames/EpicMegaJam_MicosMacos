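; Interactable lever that turns through several revolutions while engaged and winds back when released.
; A timeline drives the rotation and passes its progress to CallLeverWorkingDispatcher; a non-returning lever locks and disables interaction at full travel.
; The construction script pushes InteractionSettings into a child ChildInteractionBP and derives timeline speed from PushDuration.
; EventFakeLeverCompleted plays the same motion without the completion check.
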(event Custom|EventFakeLeverCompleted
  (bind (_direction _newtrack_0) (Timeline|Timeline_0 Play)
    (:Update
      (Transformation|SetRelativeRotation (Variables|Default|GetLever) (Math|Rotator|Lerp(Rotator) "0, 0, 0" "-1600.000000,0.000000,0.000000" _newtrack_0) false false)
      (Default|CallLeverWorkingDispatcher _newtrack_0))
    (:Finished
      (switch Utilities|FlowControl|Switch|SwitchonETimelineDirection _direction
        (:Forward
          (if (not (Variables|Default|GetLeverReturns))
            (Variables|Default|SetLeverCompleted true)
            (Default|ForceDisableInteraction (.AsChild%20Interaction%20BP (Utilities|Casting|CastToChildInteractionBP (Variables|/Script/Engine.ChildActorComponent|GetChildActor (Variables|Default|GetChildInteractionActor)))))))))))

(event EventInteractFunction
  (if (not (Variables|Default|GetLeverCompleted))
    (bind (_direction _newtrack_0) (Timeline|Timeline_0 Play)
      (:Update
        (Transformation|SetRelativeRotation (Variables|Default|GetLever) (Math|Rotator|Lerp(Rotator) "0, 0, 0" "-1600.000000,0.000000,0.000000" _newtrack_0) false false)
        (Default|CallLeverWorkingDispatcher _newtrack_0))
      (:Finished
        (switch Utilities|FlowControl|Switch|SwitchonETimelineDirection _direction
          (:Forward
            (if (not (Variables|Default|GetLeverReturns))
              (Variables|Default|SetLeverCompleted true)
              (Default|ForceDisableInteraction (.AsChild%20Interaction%20BP (Utilities|Casting|CastToChildInteractionBP (Variables|/Script/Engine.ChildActorComponent|GetChildActor (Variables|Default|GetChildInteractionActor))))))))))))

(event EventDeInteractFunction
  (if (not (Variables|Default|GetLeverCompleted))
    (bind (_direction _newtrack_0) (Timeline|Timeline_0 Reverse)
      (:Update
        (Transformation|SetRelativeRotation (Variables|Default|GetLever) (Math|Rotator|Lerp(Rotator) "0, 0, 0" "-1600.000000,0.000000,0.000000" _newtrack_0) false false)
        (Default|CallLeverWorkingDispatcher _newtrack_0))
      (:Finished
        (switch Utilities|FlowControl|Switch|SwitchonETimelineDirection _direction
          (:Forward
            (if (not (Variables|Default|GetLeverReturns))
              (Variables|Default|SetLeverCompleted true)
              (Default|ForceDisableInteraction (.AsChild%20Interaction%20BP (Utilities|Casting|CastToChildInteractionBP (Variables|/Script/Engine.ChildActorComponent|GetChildActor (Variables|Default|GetChildInteractionActor))))))))))))

(fn ConstructionScript
  (bind _childinteractionactor (Variables|Default|GetChildInteractionActor))
  (bind _childactor (Variables|/Script/Engine.ChildActorComponent|GetChildActor _childinteractionactor))
  (bind _aschild_interaction_bp (Utilities|Casting|CastToChildInteractionBP _childactor))
  (Variables|/Game/Blueprints/Interaction_BPs/ChildInteractionBP.ChildInteractionBP_C|SetInteractionStructure _aschild_interaction_bp (Variables|Default|GetInteractionSettings))
  (Default|ConstructionFunction _aschild_interaction_bp)
  (Components|Timeline|SetPlayRate (Variables|Default|GetTimeline_0) (/ 1.0 (Variables|Default|GetPushDuration))))