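; Mobile platform actor that moves between its start position and an offset set by direction (up, down, left, right) and distance, with construction-script scaling.
; A timeline, rate-scaled by travel duration, lerps the location and posts hydraulic Wwise sounds.
; It can auto-start, then ping-pongs with a return delay, or runs once with optional return.
; A reset event replays the one-shot round trip, otherwise printing an error.
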(event Custom|SetDestination
  (bind _returnvalue (Transformation|GetActorLocation))
  (bind _distance (Variables|Default|GetDistance))
  (bind (_x _y _z) (Math|Vector|BreakVector _returnvalue))
  (bind (_x_2 _y_2 _z_2) (Math|Vector|BreakVector _returnvalue))
  (bind (_x_3 _y_3 _z_3) (Math|Vector|BreakVector _returnvalue))
  (bind (_x_4 _y_4 _z_4) (Math|Vector|BreakVector _returnvalue))
  ;[1 0.269 0.9661] Set Platform Direction
  (switch Utilities|FlowControl|Switch|SwitchonDirectionsEnum (Variables|Default|GetDirection)
    (:NewEnumerator0
      (Variables|Default|SetDestination (Math|Vector|MakeVector _x_3 _y_3 (+ _z_3 _distance))))
    (:NewEnumerator1
      (Variables|Default|SetDestination (Math|Vector|MakeVector _x_4 _y_4 (- _z_4 _distance))))
    (:NewEnumerator2
      (Variables|Default|SetDestination (Math|Vector|MakeVector _x (- _y _distance) _z)))
    (:NewEnumerator3
      (Variables|Default|SetDestination (Math|Vector|MakeVector _x_2 (+ _y_2 _distance) _z_2)))))

(event Custom|TriggerMovement
  (bind _self self)
  (bind _returntime (Variables|Default|GetReturnTime))
  (bind _timeline_0 (Variables|Default|GetTimeline_0))
  (bind (_direction _movement) (Timeline|Timeline_0 Play)
    (:Update
      (Transformation|SetActorLocation (Math|Vector|Lerp(Vector) (Variables|Default|GetInitPosition) (Variables|Default|GetDestination) _movement) false false))
    (:Finished
      (Class|AkGameplayStatics|PostEvent "/Game/WwiseAudio/Events/Default_Work_Unit/Gameplay/hydraulic_end.hydraulic_end" _self)
      (if (Variables|Default|GetDoOnce)
        (if (Variables|Default|GetDoOnceReverse)
          (switch Utilities|FlowControl|Switch|SwitchonETimelineDirection _direction
            (:Forward
              (Utilities|FlowControl|Delay _returntime)
              (Components|Timeline|ReversefromEnd _timeline_0))))
        (else
          (switch Utilities|FlowControl|Switch|SwitchonETimelineDirection _direction
            (:Forward
              (Utilities|FlowControl|Delay _returntime)
              (Components|Timeline|ReversefromEnd _timeline_0))
            (:Backward
              (Utilities|FlowControl|Delay _returntime)
              (Components|Timeline|PlayfromStart _timeline_0))))))
    (:SoundForward
      (Class|AkGameplayStatics|PostEvent "/Game/WwiseAudio/Events/Default_Work_Unit/Gameplay/hydraulic_start.hydraulic_start" _self))
    (:SoundBack
      (switch Utilities|FlowControl|Switch|SwitchonETimelineDirection _direction
        (:Backward
          (Class|AkGameplayStatics|PostEvent "/Game/WwiseAudio/Events/Default_Work_Unit/Gameplay/hydraulic_start.hydraulic_start" _self))))))

(event Custom|ResetDoOnce
  (if (and (Variables|Default|GetDoOnceReverse) (Variables|Default|GetDoOnce))
    (Components|Timeline|SetNewTime (Variables|Default|GetTimeline_0) 0.0)
    (CallFunction|TriggerMovement)
    (else
      (Development|PrintString "MOBILE PLATFORM DO ONCE RESET COULD NOT BE DONE! 
Talk to Lucho, cacho tonto"))))

(event EventBeginPlay
  (Components|Timeline|SetPlayRate (Variables|Default|GetTimeline_0) (/ 1.0 (Variables|Default|GetTravelDuration)))
  (Variables|Default|SetInitPosition (Transformation|GetActorLocation))
  (CallFunction|SetDestination)
  (if (Variables|Default|GetBeginMoving)
    (CallFunction|TriggerMovement)))

(fn ConstructionScript
  (Transformation|SetRelativeScale3D (Variables|Default|GetPlatform) (Variables|Default|GetPlatformSize)))