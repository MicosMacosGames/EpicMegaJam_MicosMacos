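; Timer_BP is a countdown timer actor that shows the remaining TotalTime on a text component in the world.
; Activation, by event or optionally by a Player-tagged overlap of TempDebugBox, stores the game time, and Tick derives the remaining time from it.
; Dispatchers signal running, stopped and ended states; reaching zero fires both ended and stopped.
; The construction script sizes and spaces the two texts and previews the total.
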(event OnComponentBeginOverlap(TempDebugBox)
  (params (OverlappedComponent :type Primitive%20Component%20Object%20Reference) (OtherActor :type Actor%20Object%20Reference) (OtherComp :type Primitive%20Component%20Object%20Reference) (OtherBodyIndex :type Integer) (bFromSweep :type Boolean) (SweepResult :type Hit%20Result%20Structure%20%28by%20ref%29))
  (if (and (Actor|ActorHasTag OtherActor "Player") (Variables|Default|GetActivateWithTrigger))
    (if (not (Variables|Default|GetActivate))
      (Variables|Default|SetActivate true)
      (Variables|Default|SetCurrentTime (Utilities|Time|GetGameTimeinSeconds)))))

(event Custom|EventActivateTimer
  (if (not (Variables|Default|GetActivate))
    (Variables|Default|SetActivate true)
    (Variables|Default|SetCurrentTime (Utilities|Time|GetGameTimeinSeconds))))

(event Custom|EventStopTimer
  (Variables|Default|SetActivate false)
  (Default|CallTimerStoppedDispatcher)
  (Variables|Default|SetTimerRunning false))

(event Custom|EventStopTimerAndReset
  (params (Value :type Float%20%28single-precision%29))
  (Rendering|Components|TextRender|SetText (Variables|Default|GetTimeText) (Utilities|Text|ToText(Float) (Variables|Default|GetTotalTime) "HalfToEven" false true 2 324 2 2))
  (CallFunction|EventStopTimer))

(event EventTick
  (params (DeltaSeconds :type Float%20%28single-precision%29))
  (bind _returnvalue (Utilities|Time|GetGameTimeinSeconds))
  (bind _totaltime (Variables|Default|GetTotalTime))
  (bind _timetext (Variables|Default|GetTimeText))
  (bind _currenttime (Variables|Default|GetCurrentTime))
  (bind _returnvalue_2 (- _totaltime _returnvalue))
  (bind _returnvalue_3 (+ _returnvalue_2 _currenttime))
  (if (Variables|Default|GetActivate)
    (if (< _returnvalue_3 0.05)
      (Rendering|Components|TextRender|SetText _timetext (Utilities|Text|ToText(Float) 0.0 "HalfToEven" false true 2 324 2 2))
      (Default|CallTimerEndedDispatcher)
      (Variables|Default|SetActivate false)
      (Default|CallTimerStoppedDispatcher)
      (Variables|Default|SetTimerRunning false)
      (else
        (Rendering|Components|TextRender|SetText _timetext (Utilities|Text|ToText(Float) _returnvalue_3 "HalfToEven" false true 2 324 2 2))
        (Default|CallTimerRunningDispatcher)
        (Variables|Default|SetTimerRunning true)))))

(fn ConstructionScript
  (bind _timetext (Variables|Default|GetTimeText))
  (Rendering|Components|TextRender|SetWorldSize (Variables|Default|GetTimeText) (Variables|Default|GetFontSize))
  (Transformation|AddRelativeLocation _timetext (Math|Vector|MakeVector 0.0 0.0 (- (.Z (Math|Vector|BreakVector (Variables|/Script/Engine.SceneComponent|GetRelativeLocation (Variables|Default|GetTimeText)))) (Variables|Default|GetInterlineate))) false false)
  (Rendering|Components|TextRender|SetText _timetext (Utilities|Text|ToText(Float) (Variables|Default|GetTotalTime) "HalfToEven")))