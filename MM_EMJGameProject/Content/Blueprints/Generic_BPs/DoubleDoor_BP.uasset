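; Interactable double door that toggles open and closed, with either sliding or swinging panels.
; InteractFunction drives Timeline_0 to lerp both panels; closing a swinging door enables pushing colliders until the reverse finishes.
; If a key is needed and DoorKey is still valid, Timeline_1 animates the panels without marking the door open.
; The construction script passes InteractionSettings to a child ChildInteractionBP actor.
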(event EventBeginPlay
  (Collision|SetCollisionEnabled (Variables|Default|GetPushingCollider1) "NoCollision"))

(event EventInteractFunction
  (bind _door1 (Variables|Default|GetDoor1))
  (bind _door2 (Variables|Default|GetDoor2))
  (bind _door2_2 (Variables|Default|GetDoor2))
  (bind _door1_2 (Variables|Default|GetDoor1))
  (if (Variables|Default|GetDoorOpen)
    (Variables|Default|SetDoorOpen false)
    (if (Variables|Default|GetSlidingDoor)
      (bind (_direction _newtrack_0) (Timeline|Timeline_0 Reverse)
        (:Update
          (if (Variables|Default|GetSlidingDoor)
            (Transformation|SetRelativeLocation _door1 (Math|Vector|Lerp(Vector) "0.000000, 0,139.000000" "0.000000,117.000000,139.000000" _newtrack_0) false false)
            (Transformation|SetRelativeLocation _door2_2 (Math|Vector|Lerp(Vector) "0.000000,-145.000000,139.000000" "0.000000,-262.000000,139.000000" _newtrack_0) false false)
            (else
              (Transformation|SetRelativeLocationAndRotation _door1 (Math|Vector|Lerp(Vector) "0.000000, 0,139.000000" "-56.500000,63.000000,139.000000" _newtrack_0) (Math|Rotator|Lerp(Rotator) "0, 0, 0" "0,-70.000000, 0" _newtrack_0 true) false false)
              (Transformation|SetRelativeLocationAndRotation _door2_2 (Math|Vector|Lerp(Vector) "0.000000,-145.000000,139.000000" "-56.500000,-208.000000,139.000000" _newtrack_0) (Math|Rotator|Lerp(Rotator) "0,180.000000, 0" "0,250.000000, 0" _newtrack_0 true) false false))))
        (:Finished
          (switch Utilities|FlowControl|Switch|SwitchonETimelineDirection _direction
            (:Backward
              (Collision|SetCollisionEnabled (Variables|Default|GetPushingCollider1) "NoCollision")))))
      (else
        (Collision|SetCollisionEnabled (Variables|Default|GetPushingCollider1) "QueryAndPhysics")
        (Timeline|Timeline_0 Reverse)))
    (elif (Variables|Default|GetNeedsKey)
      (Utilities|IsValid (Variables|Default|GetDoorKey)
        (:Is%20Valid
          (bind _newtrack_0_2 (Timeline|Timeline_1 PlayFromStart)
            (:Update
              (if (Variables|Default|GetSlidingDoor)
                (Transformation|SetRelativeLocation _door1_2 (Math|Vector|Lerp(Vector) "0.000000, 0,139.000000" "0.000000,117.000000,139.000000" _newtrack_0_2) false false)
                (Transformation|SetRelativeLocation _door2 (Math|Vector|Lerp(Vector) "0.000000,-145.000000,139.000000" "0.000000,-262.000000,139.000000" _newtrack_0_2) false false)
                (else
                  (Transformation|SetRelativeRotation _door1_2 (Math|Rotator|Lerp(Rotator) "0, 0, 0" "0,-70.000000, 0" _newtrack_0_2 true) false false)
                  (Transformation|SetRelativeRotation _door2 (Math|Rotator|Lerp(Rotator) "0,180.000000, 0" "0,250.000000, 0" _newtrack_0_2 true) false false))))))
        (:Is%20Not%20Valid
          (Variables|Default|SetDoorOpen true :!label _label)
          (Timeline|Timeline_0 Play)))
      (else
        (goto _label)))))

(fn ConstructionScript
  (bind _childinteractionactor (Variables|Default|GetChildInteractionActor))
  (bind _childactor (Variables|/Script/Engine.ChildActorComponent|GetChildActor _childinteractionactor))
  (bind _aschild_interaction_bp (Utilities|Casting|CastToChildInteractionBP _childactor))
  (Variables|/Game/Blueprints/Interaction_BPs/ChildInteractionBP.ChildInteractionBP_C|SetInteractionStructure _aschild_interaction_bp (Variables|Default|GetInteractionSettings))
  (Default|ConstructionFunction _aschild_interaction_bp))