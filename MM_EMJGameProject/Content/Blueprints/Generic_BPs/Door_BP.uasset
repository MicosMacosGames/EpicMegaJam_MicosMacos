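; Interactable door that either slides or swings, toggled by interaction or driven externally by a lever.
; Timelines lerp CoreDoor for open, close and locked animations, with Wwise sounds; lever events supply their own alpha.
; A key-locked door stays shut with a HUD message while its DoorKey reference remains valid.
; A pushing collider activates while swing doors close, and the construction script passes settings to the child interaction actor.
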(event Custom|EventOpenDoorWithLever
  (params (NewTime :type Float%20%28single-precision%29))
  (bind _coredoor (Variables|Default|GetCoreDoor))
  (if (Variables|Default|GetSlidingDoor)
    (Transformation|SetRelativeLocation _coredoor (Math|Vector|Lerp(Vector) "0.000000,90.000000,0.000000" "0.000000,322.000000,0.000000" NewTime) false false)
    (else
      (Transformation|SetRelativeRotation _coredoor (Math|Rotator|Lerp(Rotator) "0,90.000000, 0" "0.000000,10.000000,0.000000" NewTime true) false false))))

(event EventBeginPlay
  (Collision|SetCollisionEnabled (Variables|Default|GetPushingCollider) "NoCollision"))

(event EventInteractFunction
  (bind _returnvalue (Game|GetPlayerCharacter 0))
  (bind _self self)
  (bind _coredoor (Variables|Default|GetCoreDoor))
  (bind _coredoor_2 (Variables|Default|GetCoreDoor))
  (bind _asplayer_bp (Utilities|Casting|CastToPlayer_BP _returnvalue))
  (bind _playerinteractionhud (Variables|/Game/Blueprints/Player_BPs/Player_BP.Player_BP_C|GetPlayerInteractionHUD _asplayer_bp))
  (if (Variables|Default|GetDoorGetsOpenedExternally)
    (Class|AkGameplayStatics|PostEvent "/Game/WwiseAudio/Events/Default_Work_Unit/Gameplay/play_door_closed.play_door_closed" self)
    (else
      (Variables|Default|SetResetLockedDoorAnimation true)
      (if (Variables|Default|GetDoorOpen)
        (Variables|Default|SetDoorOpen false)
        (if (Variables|Default|GetSlidingDoor)
          _
          (else
            (Collision|SetCollisionEnabled (Variables|Default|GetPushingCollider) "QueryAndPhysics")))
        (Class|AkGameplayStatics|PostEvent "/Game/WwiseAudio/Events/Default_Work_Unit/Gameplay/play_door_opening.play_door_opening" _self)
        (bind (_direction _newtrack_0) (Timeline|Timeline_0 Reverse)
          (:Update
            (if (Variables|Default|GetSlidingDoor)
              (Transformation|SetRelativeLocation _coredoor (Math|Vector|Lerp(Vector) "0.000000,90.000000,0.000000" "0.000000,322.000000,0.000000" _newtrack_0) false false)
              (else
                (Transformation|SetRelativeRotation _coredoor (Math|Rotator|Lerp(Rotator) "0,90.000000, 0" "0.000000,10.000000,0.000000" _newtrack_0 true) false false))))
          (:Finished
            (switch Utilities|FlowControl|Switch|SwitchonETimelineDirection _direction
              (:Backward
                (Collision|SetCollisionEnabled (Variables|Default|GetPushingCollider) "NoCollision")))))
        (elif (Variables|Default|GetNeedsKey)
          (Utilities|IsValid (Variables|Default|GetDoorKey)
            (:Is%20Valid
              (Default|ShowHUD _playerinteractionhud (Utilities|Text|ToText(String) (Variables|Default|GetLockedText)))
              (Class|AkGameplayStatics|PostEvent "/Game/WwiseAudio/Events/Default_Work_Unit/Gameplay/play_door_closed.play_door_closed" _self)
              (bind _newtrack_0_2 (Timeline|Timeline_1 PlayFromStart)
                (:Update
                  (if (Variables|Default|GetSlidingDoor)
                    (Transformation|SetRelativeLocation _coredoor_2 (Math|Vector|Lerp(Vector) "0.000000,90.000000,0.000000" "0.000000,322.000000,0.000000" _newtrack_0_2) false false)
                    (else
                      (Transformation|SetRelativeRotation _coredoor_2 (Math|Rotator|Lerp(Rotator) "0,90.000000, 0" "0.000000,10.000000,0.000000" _newtrack_0_2 true) false false))))
                (:Finished
                  (if (Variables|Default|GetResetLockedDoorAnimation)
                    (Variables|Default|SetResetLockedDoorAnimation false)
                    (Utilities|FlowControl|Delay 0.1)
                    (Components|Timeline|PlayfromStart (Variables|Default|GetTimeline_1))))))
            (:Is%20Not%20Valid
              (Default|ShowHUD _playerinteractionhud (Utilities|Text|ToText(String) (Variables|Default|GetUnlockedText)))
              (Variables|Default|SetDoorOpen true :!label _label)
              (Class|AkGameplayStatics|PostEvent "/Game/WwiseAudio/Events/Default_Work_Unit/Gameplay/play_door_opening.play_door_opening" _self)
              (Timeline|Timeline_0 Play)))
          (else
            (goto _label)))))))

(fn ConstructionScript
  (bind _childinteractionactor (Variables|Default|GetChildInteractionActor))
  (bind _childactor (Variables|/Script/Engine.ChildActorComponent|GetChildActor _childinteractionactor))
  (bind _aschild_interaction_bp (Utilities|Casting|CastToChildInteractionBP _childactor))
  (Variables|/Game/Blueprints/Interaction_BPs/ChildInteractionBP.ChildInteractionBP_C|SetInteractionStructure _aschild_interaction_bp (Variables|Default|GetInteractionSettings))
  (Default|ConstructionFunction _aschild_interaction_bp))