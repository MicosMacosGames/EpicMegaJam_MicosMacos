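; NextLevelTrigger_BP is a trigger volume that moves the player to the level named in NextLevel.
; When an actor tagged Player first overlaps the box, it disables player movement and rotation, shows a BlackFadeOut widget, then opens that level after a short delay.
; The construction script sizes the box from TriggerSize and labels a text render with the target level name.
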(event OnComponentBeginOverlap(Box)
  (params (OverlappedComponent :type Primitive%20Component%20Object%20Reference) (OtherActor :type Actor%20Object%20Reference) (OtherComp :type Primitive%20Component%20Object%20Reference) (OtherBodyIndex :type Integer) (bFromSweep :type Boolean) (SweepResult :type Hit%20Result%20Structure%20%28by%20ref%29))
  (if (Actor|ActorHasTag OtherActor "Player")
    (Utilities|FlowControl|DoOnce false
      (:Completed
        (Default|TogglePlayerMovements (.AsPlayer%20BP (Utilities|Casting|CastToPlayer_BP (Game|GetPlayerCharacter 0))) false false)
        (bind _returnvalue (UserInterface|CreateWidget "/Game/Blueprints/HUD_BPs/Fades/BlackFadeOut.BlackFadeOut_C"))
        (UserInterface|Viewport|AddtoViewport _returnvalue 1)
        (Utilities|FlowControl|Delay 2.0)
        (Game|OpenLevel(byName) (Utilities|String|StringToName (Variables|Default|GetNextLevel)))))))

(fn ConstructionScript
  (Rendering|Components|TextRender|SetText (Variables|Default|GetTextRender) (Utilities|Text|ToText(String) (Utilities|String|Append "Next Level: 
" (Variables|Default|GetNextLevel))))
  (Components|Box|SetBoxExtent (Variables|Default|GetBox) (Variables|Default|GetTriggerSize) true))