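; StandardTriggerBP is a reusable box trigger that fires an activation dispatcher when an overlapping actor carries one of its activating tags.
; Begin overlap, while Active, loops over the tag array and calls the dispatcher, through a DoOnce gate if configured to fire only once.
; Outside callers can enable, disable or reset the one-shot gate.
; The construction script sizes the collider and sets the displayed text from exposed variables.
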(event OnComponentBeginOverlap(Collider)
  (params (OverlappedComponent :type Primitive%20Component%20Object%20Reference) (OtherActor :type Actor%20Object%20Reference) (OtherComp :type Primitive%20Component%20Object%20Reference) (OtherBodyIndex :type Integer) (bFromSweep :type Boolean) (SweepResult :type Hit%20Result%20Structure%20%28by%20ref%29))
  ;[0.5684 0.9401 1] This checks the array of tags that should activate the trigger. If overlapped object has any, "TagFound" is set to true... If it is true, trigger is activated (only once if "DoOnce" is true)
  (if (Variables|Default|GetActive)
    (Variables|Default|SetTagFound false)
    (for _array_element (Variables|Default|GetActivatingTags)
      (if (Actor|ActorHasTag OtherActor _array_element)
        (Variables|Default|SetTagFound true)))
    (if (Variables|Default|GetTagFound)
      (if (Variables|Default|GetDoOnce)
        (Utilities|FlowControl|DoOnce false
          (:Completed
            _)))
      (Default|CallTriggerActivationDispatcher))))

(event Custom|ResetDoOnce
  ;[0.9149 1 0.5256] Custom Events to be called from outside
  ;[0.5684 0.9401 1] This checks the array of tags that should activate the trigger. If overlapped object has any, "TagFound" is set to true... If it is true, trigger is activated (only once if "DoOnce" is true)
  (Utilities|FlowControl|DoOnce false) ; enters at Reset
)

(event Custom|DisableTrigger
  ;[0.9149 1 0.5256] Custom Events to be called from outside
  (Variables|Default|SetActive false))

(event Custom|EnableTrigger
  ;[0.9149 1 0.5256] Custom Events to be called from outside
  (Variables|Default|SetActive true))

(fn ConstructionScript
  (Components|Box|SetBoxExtent (Variables|Default|GetCollider) (Variables|Default|GetTriggerSize) true)
  (Rendering|Components|TextRender|SetText (Variables|Default|GetText) (Variables|Default|GetDisplayedTriggerText)))