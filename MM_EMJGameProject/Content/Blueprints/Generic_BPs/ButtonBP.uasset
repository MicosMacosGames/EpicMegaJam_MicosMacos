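; Interactable button with an animated lever that notifies listeners through a dispatcher when activated.
; Interaction, normal or forced, plays a timeline that swings the lever over, then reverses it, with separate forward and return durations.
; An event track on that timeline posts the Wwise activation sound and fires the dispatcher on the forward stroke only.
; The construction script passes interaction settings to a child ChildInteractionBP actor.
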(event Custom|ForceInteraction
  (bind _timeline_0 (Variables|Default|GetTimeline_0))
  (Components|Timeline|SetPlayRate (Variables|Default|GetTimeline_0) (/ 1.0 (Variables|Default|GetForwardDuration)))
  (bind (_direction _timecurve) (Timeline|Timeline_0 PlayFromStart)
    (:Update
      (Transformation|SetRelativeRotation (Variables|Default|GetLever) (Math|Rotator|Lerp(Rotator) "0.000000,0.000000,-60.000000" "0, 0,60.000000" _timecurve) false false))
    (:Finished
      (switch Utilities|FlowControl|Switch|SwitchonETimelineDirection _direction
        (:Forward
          (Components|Timeline|SetPlayRate _timeline_0 (/ 1.0 (Variables|Default|GetReturnDuration)))
          (Components|Timeline|ReversefromEnd _timeline_0))))
    (:ButtonActivatedEvent
      (switch Utilities|FlowControl|Switch|SwitchonETimelineDirection _direction
        (:Forward
          (Class|AkGameplayStatics|PostEvent "/Game/WwiseAudio/Events/Default_Work_Unit/Gameplay/play_button_active.play_button_active" self)
          (Default|CallButtonActivatedDispatcher))))))

(event EventInteractFunction
  (bind _timeline_0 (Variables|Default|GetTimeline_0))
  (Components|Timeline|SetPlayRate (Variables|Default|GetTimeline_0) (/ 1.0 (Variables|Default|GetForwardDuration)))
  (bind (_direction _timecurve) (Timeline|Timeline_0 PlayFromStart)
    (:Update
      (Transformation|SetRelativeRotation (Variables|Default|GetLever) (Math|Rotator|Lerp(Rotator) "0.000000,0.000000,-60.000000" "0, 0,60.000000" _timecurve) false false))
    (:Finished
      (switch Utilities|FlowControl|Switch|SwitchonETimelineDirection _direction
        (:Forward
          (Components|Timeline|SetPlayRate _timeline_0 (/ 1.0 (Variables|Default|GetReturnDuration)))
          (Components|Timeline|ReversefromEnd _timeline_0))))
    (:ButtonActivatedEvent
      (switch Utilities|FlowControl|Switch|SwitchonETimelineDirection _direction
        (:Forward
          (Class|AkGameplayStatics|PostEvent "/Game/WwiseAudio/Events/Default_Work_Unit/Gameplay/play_button_active.play_button_active" self)
          (Default|CallButtonActivatedDispatcher))))))

(fn ConstructionScript
  (bind _childinteractionactor (Variables|Default|GetChildInteractionActor))
  (bind _childactor (Variables|/Script/Engine.ChildActorComponent|GetChildActor _childinteractionactor))
  (bind _aschild_interaction_bp (Utilities|Casting|CastToChildInteractionBP _childactor))
  (Variables|/Game/Blueprints/Interaction_BPs/ChildInteractionBP.ChildInteractionBP_C|SetInteractionStructure _aschild_interaction_bp (Variables|Default|GetInteractionSettings))
  (Default|ConstructionFunction _aschild_interaction_bp))