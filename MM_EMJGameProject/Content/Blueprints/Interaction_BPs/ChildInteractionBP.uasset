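; Child-actor interaction component that makes its parent actor interactable, forwarding interactions to it through InteractFunction.
; An InteractionStructure configures the look-at sphere, glow box, prompt text, optional one-shot use and temporary deactivation.
; Player overlap with GlowBox toggles custom depth on name-matched parent meshes, using stencil values for glow color.
; Setup lives in ConstructionFunction because the construction script is not called from parents or children.
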(event OnComponentBeginOverlap(GlowBox)
  (params (OverlappedComponent :type Primitive%20Component%20Object%20Reference) (OtherActor :type Actor%20Object%20Reference) (OtherComp :type Primitive%20Component%20Object%20Reference) (OtherBodyIndex :type Integer) (bFromSweep :type Boolean) (SweepResult :type Hit%20Result%20Structure%20%28by%20ref%29))
  ;[0.5354 0.8478 1] On Begin/End Overlap, activate Glow + Custom Events to Activate/Deactivate Glow
  (if (or (.InteractionEnabled (Utilities|Struct|BreakInteractionStruct (Variables|Default|GetInteractionStructure))) (Variables|Default|GetTemporaryDisabled))
    (if (Actor|ActorHasTag OtherActor "Player")
      (for _array_element (Variables|Default|GetGlowingMeshes)
        (Rendering|SetRenderCustomDepth _array_element true)))))

(event OnComponentEndOverlap(GlowBox)
  (params (OverlappedComponent :type Primitive%20Component%20Object%20Reference) (OtherActor :type Actor%20Object%20Reference) (OtherComp :type Primitive%20Component%20Object%20Reference) (OtherBodyIndex :type Integer))
  ;[0.5354 0.8478 1] On Begin/End Overlap, activate Glow + Custom Events to Activate/Deactivate Glow
  (if (or (.InteractionEnabled (Utilities|Struct|BreakInteractionStruct (Variables|Default|GetInteractionStructure))) (Variables|Default|GetTemporaryDisabled))
    (if (Actor|ActorHasTag OtherActor "Player")
      (for _array_element (Variables|Default|GetGlowingMeshes)
        (Rendering|SetRenderCustomDepth _array_element false)))))

(event Custom|ResetInteraction_DoOnce
  ;[0.5865 1 0.6617] On Interaction (when the player interacts with the input)
  (Utilities|FlowControl|DoOnce false) ; enters at Reset
)

(event Custom|ShowInteractionHUD
  (bind _interactionstructure (Variables|Default|GetInteractionStructure))
  (bind (_interactionenabled _doonce _lookatsphereradius _inputtointeracttext _interactiontext) (Utilities|Struct|BreakInteractionStruct _interactionstructure))
  ;[1 1 1] Show HUD on Interaction
  (Utilities|FlowControl|DoOnce false
    (:Completed
      (Default|ShowHUD (Variables|/Game/Blueprints/Player_BPs/Player_BP.Player_BP_C|GetPlayerInteractionHUD (.AsPlayer%20BP (Utilities|Casting|CastToPlayer_BP (Game|GetPlayerCharacter 0)))) (Utilities|Text|ToText(String) (Utilities|String|Append _inputtointeracttext " | " _interactiontext))))))

(event Custom|ResetShowHUD_DoOnce
  (bind _interactionstructure (Variables|Default|GetInteractionStructure))
  (bind (_interactionenabled _doonce _lookatsphereradius _inputtointeracttext _interactiontext) (Utilities|Struct|BreakInteractionStruct _interactionstructure))
  ;[1 1 1] Show HUD on Interaction
  (Utilities|FlowControl|DoOnce false) ; enters at Reset
)

(event Custom|EndInteractionGlow
  ;[0.5354 0.8478 1] On Begin/End Overlap, activate Glow + Custom Events to Activate/Deactivate Glow
  (for _array_element (Variables|Default|GetGlowingMeshes)
    (Rendering|SetRenderCustomDepth _array_element false)))

(event Custom|BeginInteractionGlow
  ;[0.5354 0.8478 1] On Begin/End Overlap, activate Glow + Custom Events to Activate/Deactivate Glow
  (for _array_element (Variables|Default|GetGlowingMeshes)
    (Rendering|SetRenderCustomDepth _array_element true)))

(event Custom|EnableInteractionAgain
  (CallFunction|ResetInteractionDoOnce)
  (Collision|SetCollisionEnabled (Variables|Default|GetSphere) "QueryAndPhysics")
  (Utilities|Struct|SetmembersinInteractionStruct (Variables|Default|GetInteractionStructure) true)
  (CallFunction|BeginInteractionGlow))

(event Custom|TemporaryDeactivate
  (params (Duration :type Float%20%28single-precision%29))
  (bind _interactionstructure (Variables|Default|GetInteractionStructure))
  (bind _glowingmeshes (Variables|Default|GetGlowingMeshes))
  (bind (_interactionenabled _doonce _lookatsphereradius _inputtointeracttext _interactiontext _holdtointeract _glowboxsize _glowcolor) (Utilities|Struct|BreakInteractionStruct _interactionstructure))
  (Variables|Default|SetTemporaryDisabled true)
  (Variables|Default|SetInitInteractText _inputtointeracttext)
  (Variables|Default|SetInitialGlowColor (Math|Conversions|ToInteger(Byte) _glowcolor))
  (Utilities|Struct|SetmembersinInteractionStruct _interactionstructure false "Deactivated")
  (for _array_element _glowingmeshes
    (Rendering|SetCustomDepthStencilValue _array_element 3))
  (Utilities|FlowControl|Delay Duration)
  (Utilities|Struct|SetmembersinInteractionStruct _interactionstructure true (Variables|Default|GetInitInteractText))
  (for _array_element_2 _glowingmeshes
    (Rendering|SetCustomDepthStencilValue _array_element_2 (+ (Variables|Default|GetInitialGlowColor) 1))
    (Variables|Default|SetTemporaryDisabled false)
    (Default|HideHUD (Variables|/Game/Blueprints/Player_BPs/Player_BP.Player_BP_C|GetPlayerInteractionHUD (.AsPlayer%20BP (Utilities|Casting|CastToPlayer_BP (Game|GetPlayerCharacter 0)))))
    (CallFunction|ResetShowHUDDoOnce)))

(event Custom|ForceOverlapCheck
  ;[0.5354 0.8478 1] On Begin/End Overlap, activate Glow + Custom Events to Activate/Deactivate Glow
  (if (or (.InteractionEnabled (Utilities|Struct|BreakInteractionStruct (Variables|Default|GetInteractionStructure))) (Variables|Default|GetTemporaryDisabled))
    (if (Actor|ActorHasTag (stale OnComponentBeginOverlap(GlowBox) OtherActor) "Player")
      (for _array_element (Variables|Default|GetGlowingMeshes)
        (Rendering|SetRenderCustomDepth _array_element true)))))

(event EventInteractFunction
  (bind _interactionstructure (Variables|Default|GetInteractionStructure))
  (bind (_interactionenabled _doonce _lookatsphereradius _inputtointeracttext _interactiontext) (Utilities|Struct|BreakInteractionStruct _interactionstructure))
  ;[0.5865 1 0.6617] On Interaction (when the player interacts with the input)
  (if _interactionenabled
    (if _doonce
      (Utilities|FlowControl|DoOnce false
        (:Completed
          (CallFunction|EndInteractionGlow)
          (Collision|SetCollisionEnabled (Variables|Default|GetSphere) "NoCollision")
          (Utilities|Struct|SetmembersinInteractionStruct (Variables|Default|GetInteractionStructure) false))))
    (Class|InteractionInterfaceBP|InteractFunction(Message) (Actor|GetParentActor))))

(fn ConstructionScript
  ;[1 0.01085 0] DON'T USE THIS, IT'S NOT CALLED FROM CHILDS/PARENTS!!! Use "Construction Function" Instead!!!!!!!!!!!
)

(fn ConstructionFunction
  (bind _interactionstructure (Variables|Default|GetInteractionStructure))
  (bind (_interactionenabled _doonce _lookatsphereradius _inputtointeracttext _interactiontext _holdtointeract _glowboxsize _glowcolor _glowmeshesname) (Utilities|Struct|BreakInteractionStruct _interactionstructure))
  ;[1 1 1] Setup of class variables (interaction sphere radius, glow box size, displayed debug text ...)
  (Variables|Default|SetInitInteractText _inputtointeracttext)
  (Variables|Default|SetInitialGlowColor (Math|Conversions|ToInteger(Byte) _glowcolor))
  (Components|Sphere|SetSphereRadius (Variables|Default|GetSphere) _lookatsphereradius true)
  (Components|Box|SetBoxExtent (Variables|Default|GetGlowBox) _glowboxsize true)
  (Rendering|Components|TextRender|SetText (Variables|Default|GetInteractionObjectText) (Variables|Default|GetInteractionObjectTextDisplay))
  ;[0.8435 0.7671 1] Set Meshes to Glow on Interaction
  (for _array_element (Actor|GetComponentsByClass (Actor|GetParentActor) "/Script/Engine.StaticMeshComponent")
    (for _array_element_2 _glowmeshesname
      (if (Utilities|String|Contains (Utilities|GetDisplayName _array_element) _array_element_2)
        (Utilities|Array|Add (Variables|Default|GetGlowingMeshes) _array_element))))
  (for _array_element_3 (Variables|Default|GetGlowingMeshes)
    (switch Utilities|FlowControl|Switch|SwitchonGlowColorEnum _glowcolor
      (:NewEnumerator0
        (Rendering|SetCustomDepthStencilValue _array_element_3 1))
      (:NewEnumerator1
        (Rendering|SetCustomDepthStencilValue _array_element_3 2))
      (:NewEnumerator2
        (Rendering|SetCustomDepthStencilValue _array_element_3 3))
      (:NewEnumerator3
        (Rendering|SetCustomDepthStencilValue _array_element_3 4)))))